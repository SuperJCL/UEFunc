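; Spline polyline actor that draws a styled path or trail wall from an array of longitude, latitude and height points.
; CreatSpline converts the points to world positions, rebuilds the spline, adds a spline mesh per segment and returns the spline length.
; Mesh direction (centered, side-aligned, standing) selects mesh and axes, while style picks a StyleLibrary material.
; Dynamic material instances set color, brightness, scroll speed, stroke, and tiling scaled by segment length.
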(fn `Creat Spline`
  (params (positionArray :type "Array of /Game/functions/camera/positionStruct Structure") (color :type "Color Structure") (width :type "Float (double-precision)") (brightness :type "Float (double-precision)") (tilling :type "Float (double-precision)") (speed :type "Float (double-precision)") (openStroke :type Boolean) (strokeWidth :type "Float (double-precision)") (style :type String) (meshDirection :type String) (pathColorR :type "Float (double-precision)") (pathColorG :type "Float (double-precision)") (pathColorB :type "Float (double-precision)") (pathColorA :type "Float (double-precision)"))
  (returns (splineLength :type "Float (double-precision)"))
  (bind _returnvalue (`KismetMathLibrary.MakeVector` 0.0 0.0 1.0))
  (bind _speed (`self.Speed`))
  (bind _meshdirection (`self.MeshDirection`))
  (bind _tilling (`self.Tilling`))
  (bind _meshdirection_2 (`self.MeshDirection`))
  (bind (_color_r _color_g _color_b _color_a) (break `LinearColor` (`self.Color`)))
  (bind _spline (`self.Spline`))
  (bind _splinetangent_0 (`self.SplineTangent=0`))
  (bind _returnvalue_2 (/ (`self.Width`) 50.0))
  (bind _value (`BlueprintMapLibrary.Map_Find` (`self.Style_library`) (`|GetEnumeratorNameAsString` (`self.Style`))))
  ;[1 1 1] 处理样条点数组
  (set `self.PositionVectorArray` (`self.NullVectorArray`))
  (for (_array_element _array_index) positionArray
    (bind _data (`/Game/functions/utils/coordinate.经纬度转ue` (break `/Game/functions/camera/positionStruct` _array_element) (`.lat_14_DA33F52244211687C8D95CA22928C130` (break `/Game/functions/camera/positionStruct` _array_element)) (`.height_15_83ACDBEF44BE26100B029BB939BE2653` (break `/Game/functions/camera/positionStruct` _array_element))))
    (`KismetArrayLibrary.Array_Insert` (`self.PositionVectorArray`) (`KismetMathLibrary.MakeVector` (.x _data) (.y _data) (.z _data)) _array_index))
  ;[1 1 1] 颜色
  (set `self.Color` (make `LinearColor` pathColorR pathColorG pathColorB pathColorA))
  ;[1 1 1] 宽度
  (set `self.Width` width)
  ;[1 1 1] 亮度
  (set `self.Brightness` brightness)
  ;[1 1 1] 纹理平铺
  (set `self.Tilling` tilling)
  ;[1 1 1] 速度
  (set `self.Speed` speed)
  ;[1 1 1] 开启描边
  (set `self.Open_Stroke` openStroke)
  ;[1 1 1] 描边宽度
  (set `self.Stroke_Width` strokeWidth)
  ;[1 1 1] 轨迹墙风格
  (switch `string` style
    (:`纯色`
      (set `self.Style` "NewEnumerator0"))
    (:`虚线`
      (set `self.Style` "NewEnumerator1"))
    (:`箭头`
      (set `self.Style` "NewEnumerator2"))
    (:`渐变`
      (set `self.Style` "NewEnumerator3"))
    (:`定制`
      (set `self.Style` "NewEnumerator6")))
  ;[1 1 1] 模型朝向
  (switch `string` meshDirection
    (:`居中`
      (set `self.MeshDirection` "NewEnumerator0"))
    (:`贴边`
      (set `self.MeshDirection` "NewEnumerator3"))
    (:`站立`
      (set `self.MeshDirection` "NewEnumerator1")))
  ;[1 1 1] 绘制样条点
  (`SplineComponent.ClearSplinePoints` (`self.Spline`) true) ; 清除样条点
  (for _array_element_2 (`self.PositionVectorArray`)
    (`SplineComponent.AddSplinePoint` (`self.Spline`) _array_element_2 "World" true))
  (for _index (range (+ (- (`SplineComponent.GetNumberOfSplinePoints` (`self.Spline`)) (select `bool` (`self.Loop`) :`false` 2 :`true` 1)) 1))
    (`SplineComponent.SetSplinePointType` (`self.Spline`) _index (`self.Spline_Type`) true) ; 设置样条线的类型
    (bind _returnvalue_3 (`AddComponent|NODE_AddSplineMeshComponent-8`))
    (`StaticMeshComponent.SetStaticMesh` _returnvalue_3 (select `/Game/AssetsLibrary/4_BPTools/SplineTools/Spline_Polyline/Enum/E_PolyLine_Direction` _meshdirection :`NewEnumerator0` "/Game/AssetsLibrary/4_BPTools/SplineTools/Spline_Polyline/Mesh/plane_Center.plane_Center" :`NewEnumerator3` "/Game/AssetsLibrary/4_BPTools/SplineTools/Spline_Polyline/Mesh/Plane_Side.Plane_Side" :`NewEnumerator1` "/Game/AssetsLibrary/4_BPTools/SplineTools/Spline_Polyline/Mesh/plane_Center.plane_Center" :!type "StaticMesh Object Reference"))
    (`SplineMeshComponent.SetForwardAxis` _returnvalue_3 (select `/Game/AssetsLibrary/4_BPTools/SplineTools/Spline_Polyline/Enum/E_PolyLine_Direction` _meshdirection :`NewEnumerator0` "X" :`NewEnumerator3` "X" :`NewEnumerator1` "Y" :!type "ESplineMeshAxis Enum") true)
    (`SplineMeshComponent.SetSplineUpDir` _returnvalue_3 (select `/Game/AssetsLibrary/4_BPTools/SplineTools/Spline_Polyline/Enum/E_PolyLine_Direction` _meshdirection :`NewEnumerator0` _returnvalue :`NewEnumerator3` _returnvalue :`NewEnumerator1` (`KismetMathLibrary.MakeVector` 0.0 0.0 -1.0)) true)
    (`SplineMeshComponent.SetStartScale` _returnvalue_3 (`KismetMathLibrary.MakeVector2D` _returnvalue_2 _returnvalue_2) true)
    (`SplineMeshComponent.SetEndScale` _returnvalue_3 (`KismetMathLibrary.MakeVector2D` _returnvalue_2 _returnvalue_2) true)
    (`PrimitiveComponent.SetMassScale` _returnvalue_3 "None" 1.0)
    (`/Engine/EditorBlueprintResources/StandardMacros.IsValid` _value
      (:`Is Valid`
        (bind _returnvalue_4 (`PrimitiveComponent.CreateDynamicMaterialInstance` _returnvalue_3 0 _value "None"))
        (`MaterialInstanceDynamic.SetScalarParameterValue` _returnvalue_4 "E_Brightness" (`self.Brightness`))
        (`MaterialInstanceDynamic.SetVectorParameterValue` _returnvalue_4 "E_Color" (make `LinearColor` _color_r _color_g _color_b _color_a))
        (`MaterialInstanceDynamic.SetScalarParameterValue` _returnvalue_4 (select `/Game/AssetsLibrary/4_BPTools/SplineTools/Spline_Polyline/Enum/E_PolyLine_Direction` _meshdirection_2 :`NewEnumerator0` "SpeedY" :`NewEnumerator3` "SpeedX" :`NewEnumerator1` "SpeedX" :!type "Name") (select `/Game/AssetsLibrary/4_BPTools/SplineTools/Spline_Polyline/Enum/E_PolyLine_Direction` (`self.MeshDirection`) :`NewEnumerator0` _speed :`NewEnumerator3` (* _speed -1.0) :`NewEnumerator1` _speed))
        (`MaterialInstanceDynamic.SetScalarParameterValue` _returnvalue_4 "UV_Rotation" (select `/Game/AssetsLibrary/4_BPTools/SplineTools/Spline_Polyline/Enum/E_PolyLine_Direction` _meshdirection_2 :`NewEnumerator3` -0.25 :`NewEnumerator1` -0.25))
        (bind (_location _tangent) (`SplineComponent.GetLocationAndTangentAtSplinePoint` _spline _index "Local"))
        (bind (_location_2 _tangent_2) (`SplineComponent.GetLocationAndTangentAtSplinePoint` _spline (+ _index 1) "Local"))
        (`MaterialInstanceDynamic.SetScalarParameterValue` _returnvalue_4 (select `/Game/AssetsLibrary/4_BPTools/SplineTools/Spline_Polyline/Enum/E_PolyLine_Direction` _meshdirection_2 :`NewEnumerator0` "V" :`NewEnumerator3` "U" :`NewEnumerator1` "U" :!type "Name") (/ (`KismetMathLibrary.VSize` (- _location _location_2)) (select `/Game/AssetsLibrary/4_BPTools/SplineTools/Spline_Polyline/Enum/E_PolyLine_Direction` (`self.MeshDirection`) :`NewEnumerator0` (* _tilling -1.0) :`NewEnumerator3` _tilling :`NewEnumerator1` _tilling)))
        (`MaterialInstanceDynamic.SetScalarParameterValue` _returnvalue_4 "Stroke_Swich" (select `bool` (`self.Open_Stroke`) :`true` 1.0))
        (`MaterialInstanceDynamic.SetScalarParameterValue` _returnvalue_4 "Stroke_Width" (`KismetMathLibrary.MapRangeClamped` (`self.Stroke_Width`) 0.0 1.0 0.999 1.0002))
        (`SceneComponent.K2_AttachToComponent` _returnvalue_3 (`self.Spline`) "None" "KeepRelative" "KeepRelative" "KeepRelative" true)
        (`SplineMeshComponent.SetStartAndEnd` _returnvalue_3 _location (select `bool` _splinetangent_0 :`false` _tangent) _location_2 (select `bool` _splinetangent_0 :`false` _tangent_2 :`true` (1.0 0.0 0.0)) true))))
  ;[1 1 1] 绘制完成返回
  (return (`SplineComponent.GetSplineLength` (`self.Spline`))))

(fn `UserConstructionScript`
  (`SplineComponent.SetClosedLoop` (`self.Spline`) (`self.Loop`) true))